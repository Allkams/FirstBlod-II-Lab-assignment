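; HUD Blueprint for the FirstBlood tutorial that draws a color-mode screen overlay and a coin score counter.
; Each DrawHUD stretches a green or red material across the screen based on GreenMode and RedMode, falling back to blue.
; The blue branch's condition is hard-wired true, so its BlueMode assignment never runs.
; It then draws a coin icon and the Score value at the top right, offset from the screen width.
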(event `self.ReceiveDrawHUD`
  (params (SizeX :type Integer) (SizeY :type Integer))
  (set `self.Size X` SizeX)
  (set `self.Size Y` SizeY)
  (`|ExecutionSequence`
    (:`then_0`
      (if (`self.GreenMode`)
        (`self.DrawMaterialSimple` "/Game/Tut_FirstBlood/Materials/MAT_Hud_Green.MAT_Hud_Green" 0.0 0.0 (`KismetMathLibrary.Conv_IntToDouble` (`self.Size X`)) (`KismetMathLibrary.Conv_IntToDouble` (`self.Size Y`)))
        (elif (`self.RedMode`)
          (`self.DrawMaterialSimple` "/Game/Tut_FirstBlood/Materials/MAT_Hud_Red.MAT_Hud_Red" 0.0 0.0 (`KismetMathLibrary.Conv_IntToDouble` (`self.Size X`)) (`KismetMathLibrary.Conv_IntToDouble` (`self.Size Y`)))
          (elif true
            (`self.DrawMaterialSimple` "/Game/Tut_FirstBlood/Materials/MAT_Hud_Blue.MAT_Hud_Blue" 0.0 0.0 (`KismetMathLibrary.Conv_IntToDouble` (`self.Size X`)) (`KismetMathLibrary.Conv_IntToDouble` (`self.Size Y`)))
            (else
              (set `self.BlueMode` true))))))
    (:`then_1`
      (`self.DrawMaterialSimple` "/Game/Tut_FirstBlood/Materials/MAT_Coin.MAT_Coin" (- (`KismetMathLibrary.Conv_IntToDouble` (`self.Size X`)) 250.0) 100.0 100.0 100.0)
      (`self.DrawText` "x" (struct :`R` 1.0 :`G` 1.0 :`B` 1.0 :`A` 1.0) (- (`KismetMathLibrary.Conv_IntToDouble` (`self.Size X`)) 150.0) 120.0 "/Engine/EngineFonts/RobotoDistanceField.RobotoDistanceField" 2.5)
      (`self.DrawText` (`KismetStringLibrary.Conv_IntToString` (`self.Score`)) (struct :`R` 1.0 :`G` 1.0 :`B` 1.0 :`A` 1.0) (- (`KismetMathLibrary.Conv_IntToDouble` (`self.Size X`)) 110.0) 120.0 "/Engine/EngineFonts/RobotoDistanceField.RobotoDistanceField" 2.5))))

(fn `UserConstructionScript`)